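; Game mode Blueprint that puts the UI widget on screen and prints the chat lines from DT_Chat when play begins.
; BeginPlay runs a sequence that creates and stores the widget, gets the table's row names, then loops from 1 to the row count.
; Each index becomes a row name via string conversion, so only numerically named rows are found and printed as "Name : Sentence".
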(event EventBeginPlay
  (Utilities|FlowControl|Sequence
    (:then_0
      (bind _returnvalue (UserInterface|CreateWidget "/Game/BluePrint/UI.UI_C"))
      (bind _output_get (Variables|Default|SetNewVar _returnvalue))
      (UserInterface|Viewport|AddtoViewport _output_get 0))
    (:then_1
      ;[1 1 1] Data Table 크기 반환
      (bind _outrownames (DataTable|GetDataTableRowNames "/Game/BluePrint/DT_Chat.DT_Chat")))
    (:then_2
      ;[1 1 1] For with Break
      (bind _index (Utilities|FlowControl|ForLoopwithBreak 1 (Utilities|Array|Length _outrownames))
        (:LoopBody
          ;[1 1 1] Data Table 참조
          (bind _returnvalue_2 (Utilities|GetDataTableRow "/Game/BluePrint/DT_Chat.DT_Chat" (Utilities|String|StringToName (Utilities|String|ToString(Integer) _index)))
            (:then
              (Development|PrintString (Utilities|String|ToString(Text) (Utilities|Text|FormatText "{0} : {1}" (.Name (Utilities|Struct|BreakST_Chatdata _returnvalue_2)) (.Sentence (Utilities|Struct|BreakST_Chatdata _returnvalue_2))))))))))))

(event EventTick
  (params (DeltaSeconds :type Float%20%28single-precision%29)))

(fn ConstructionScript)